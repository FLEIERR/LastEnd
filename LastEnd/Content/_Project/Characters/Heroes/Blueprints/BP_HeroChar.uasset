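; Playable hero character whose mesh comes from a data table row chosen in the game instance, defaulting to Manny.
; Running requires forward input and turns toward movement, with a LookForward timeline easing yaw back to the camera afterward.
; Jumping while running plays a roll montage and temporarily shrinks the capsule.
; Pausing blends the view to a child-actor camera and shows an in-world menu widget driven by WidgetInteraction.
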(event `InputAction|PauseInput`
  (params (Key :type "Key Structure"))
  (:`Pressed`
    (if (`self.openPauseMenu?`)
      (`self.Resume Game Menu`)
      (else
        (`self.Pause Game Menu`)
        ;[1 1 1] Test
        (set `self.openPauseMenu?` true)))))

(event `Pause Game Menu`
  (bind _returnvalue (`GameplayStatics.GetPlayerController` 0))
  ;[1 1 1] Test
  (`PlayerController.SetViewTargetWithBlend` (`GameplayStatics.GetPlayerController` 0) (`ChildActorComponent.ChildActor` (`self.Camera Target`)) 0.2 "VTBlend_Linear" 0.0 false)
  (`SceneComponent.SetHiddenInGame` (`self.WidgetInteraction`) false false)
  (`SceneComponent.SetHiddenInGame` (`self.Widget`) false false)
  (`WidgetBlueprintLibrary.SetInputMode_UIOnlyEx` _returnvalue (`WidgetComponent.GetWidget` (`self.Widget`)))
  (set `PlayerController.bShowMouseCursor` true _returnvalue)
  (`WidgetInteractionComponent.SetFocus` (`self.WidgetInteraction`) (`WidgetComponent.GetWidget` (`self.Widget`))))

(event `self.ReceiveBeginPlay`
  (bind _returnvalue (`GameplayStatics.GetPlayerController` 0))
  (`|ExecutionSequence`
    (:`then_0`
      (`self.SetCharacterInfos`)
      (`WidgetBlueprintLibrary.SetInputMode_GameOnly` _returnvalue)
      (set `PlayerController.bShowMouseCursor` false _returnvalue)
      (set `self.capsuleSize` (`CapsuleComponent.CapsuleHalfHeight` (`self.CapsuleComponent`))))
    (:`then_1`
      (set `self.defaultCharacterSpeed` (`CharacterMovementComponent.MaxWalkSpeed` (`self.CharacterMovement`))))))

(event `Key|LeftMouseButton`
  (params (Key :type "Key Structure"))
  ;[1 1 1] Test
  (:`Pressed`
    (`WidgetInteractionComponent.PressPointerKey` (`self.WidgetInteraction`) (stale `self.Widget.OnClicked` ButtonPressed) :!label _label)))

(event `self.Widget.OnClicked`
  (params (TouchedComponent :type "PrimitiveComponent Object Reference") (ButtonPressed :type "Key Structure"))
  ;[1 1 1] Test
  (goto _label))

(event `Resume Game Menu`
  (bind _returnvalue (`GameplayStatics.GetPlayerController` 0))
  ;[1 1 1] Test
  (`PlayerController.SetViewTargetWithBlend` (`GameplayStatics.GetPlayerController` 0) self 0.2 "VTBlend_Linear" 0.0 false)
  (`SceneComponent.SetHiddenInGame` (`self.WidgetInteraction`) true false)
  (`SceneComponent.SetHiddenInGame` (`self.Widget`) true false)
  (`WidgetBlueprintLibrary.SetInputMode_GameOnly` _returnvalue)
  (set `PlayerController.bShowMouseCursor` false _returnvalue)
  (set `self.openPauseMenu?` false))

(event `self.ReceiveActorBeginOverlap`
  (params (OtherActor :type "Actor Object Reference")))

(event `InputAxis|MoveFWD`
  (params (AxisValue :type "Float (single-precision)"))
  (`self.AddMovementInput` (`KismetMathLibrary.GetForwardVector` (`KismetMathLibrary.MakeRotator` 0.0 0.0 (.yaw (`self.GetControlRotation`)))) AxisValue))

(event `InputAxis|LookUp`
  (params (AxisValue :type "Float (single-precision)"))
  (`self.AddControllerPitchInput` AxisValue))

(event `InputAxis|Turn`
  (params (AxisValue :type "Float (single-precision)"))
  (`self.AddControllerYawInput` AxisValue))

(event `InputAxis|MoveRGT`
  (params (AxisValue :type "Float (single-precision)"))
  (`self.AddMovementInput` (`KismetMathLibrary.GetRightVector` (`KismetMathLibrary.MakeRotator` 0.0 0.0 (.yaw (`self.GetControlRotation`)))) AxisValue))

(event `self.ReceiveTick`
  (params (DeltaSeconds :type "Float (single-precision)"))
  (`KismetSystemLibrary.PrintString` (`KismetStringLibrary.Conv_BoolToString` (`self.isRunning?`)) true true (struct :`R` 1.0 :`G` 0.062871 :`A` 1.0) 0.0)
  (`|ExecutionSequence`
    (:`then_0`
      (bind _canrun_ (`self.CheckCanRun`))
      (bind _output_get (set `self.Can Run?` _canrun_))
      (if _output_get
        (goto _label_2 :!via `Reset`)
        (else
          (set `CharacterMovementComponent.bOrientRotationToMovement` false (`self.CharacterMovement`))
          (set `self.isRunning?` false)
          (`/Engine/EditorBlueprintResources/StandardMacros.DoOnce` false :!label _label_2
            (:`Completed`
              (`TimelineComponent.Play` (`self.LookForward`)))))))
    (:`then_1`
      (if (`self.isPlayingRollMontage?`)
        (bind _output_get_2 (set `self.bUseControllerRotationYaw` false))
        (`KismetSystemLibrary.PrintString` (`KismetStringLibrary.Conv_BoolToString` _output_get_2) true true (struct :`R` 1.0 :`B` 0.887786 :`A` 1.0))
        (`TimelineComponent.Stop` (`self.LookForward`))))))

(event `InputAction|Run`
  (params (Key :type "Key Structure"))
  (bind _charactermovement (`self.CharacterMovement`))
  (bind _lookforward (`self.LookForward`))
  (bind _charactermovement_2 (`self.CharacterMovement`))
  (:`Pressed`
    (if (`self.Can Run?`)
      (set `CharacterMovementComponent.MaxWalkSpeed` (`self.RunSpeed`) _charactermovement)
      (set `self.bUseControllerRotationYaw` false)
      (set `CharacterMovementComponent.bOrientRotationToMovement` true _charactermovement)
      (`KismetSystemLibrary.PrintString` "Hello")
      (set `self.isRunning?` true)
      (`TimelineComponent.Stop` _lookforward)
      (`TimelineComponent.SetNewTime` _lookforward 0.0)))
  (:`Released`
    (set `CharacterMovementComponent.MaxWalkSpeed` (`self.defaultCharacterSpeed`) _charactermovement_2)
    (set `CharacterMovementComponent.bOrientRotationToMovement` false _charactermovement_2)
    (set `self.isRunning?` false)
    (if (not (`self.isPlayingRollMontage?`))
      (`TimelineComponent.Play` (`self.LookForward`)))))

(event `InputAction|Jump`
  (params (Key :type "Key Structure"))
  (:`Pressed`
    (if (`self.isRunning?`)
      (if (not (`self.isPlayingRollMontage?`))
        (`self.Jump`)
        (`|PlayMontage` (`self.Mesh`) "/Game/_Project/Characters/Heroes/Animations/FromMixamo/BigJump_Montage.BigJump_Montage"
          (:`then`
            (`KismetSystemLibrary.PrintString` "JUMP")
            (set `self.isPlayingRollMontage?` true)
            (`CapsuleComponent.SetCapsuleHalfHeight` (`self.CapsuleComponent`) 10.0 true)
            (bind _returnvalue (`AnimSequenceBase.GetPlayLength` (`self.GetCurrentMontage`)))
            (`KismetSystemLibrary.Delay` (- _returnvalue 0.3))
            (`CapsuleComponent.SetCapsuleHalfHeight` (`self.CapsuleComponent`) (`self.capsuleSize`) true))
          (:`OnCompleted`
            (set `self.isPlayingRollMontage?` false)
            (`TimelineComponent.PlayFromStart` (`self.LookForward`)))))
      (else
        (`KismetSystemLibrary.PrintString` "NOT JUMP")
        (`self.Jump`))))
  (:`Released`
    (`self.StopJumping`)))

(fn `CheckCanRun`
  (returns (`CanRun?` :type Boolean))
  (if (> (`self.GetInputAxisValue`) 0.0)
    (return true)
    (else
      (return false))))

(fn `GetMyGameInstance`
  (returns (`AsGame Instance Hero Char` :type "/Game/_Project/Characters/Heroes/Blueprints/GameInstance_HeroChar Object Reference"))
  (bind _asgame_instance_hero_char (cast `/Game/_Project/Characters/Heroes/Blueprints/GameInstance_HeroChar` (`GameplayStatics.GetGameInstance`)))
  (return _asgame_instance_hero_char))

(fn `SetCharacterInfos`
  (bind _asgame_instance_hero_char (`self.GetMyGameInstance`))
  (if (== (`/Game/_Project/Characters/Heroes/Blueprints/GameInstance_HeroChar.CharacterDataRow` _asgame_instance_hero_char) "None")
    (bind _returnvalue (`|GetDataTableRow` "/Game/_Project/Characters/Heroes/DataTables/Rows/DataTabel_Character.DataTabel_Character" "Manny")
      (:`then`
        (bind (_charactermesh _charactername _animmenu) (break `/Game/_Project/Characters/Heroes/DataTables/Struct_Characters` _returnvalue))
        (set `self.Character Mesh` _charactermesh)
        (set `self.Character Name` _charactername)
        (set `self.Anim Menu` _animmenu)
        (`SkinnedMeshComponent.SetSkinnedAssetAndUpdate` (`self.Mesh`) (`self.Character Mesh`) true :!label _label)
        (return))
      (:`RowNotFound`
        (`KismetSystemLibrary.PrintString` "Something Went Wrong")))
    (else
      (bind _returnvalue_2 (`|GetDataTableRow` "/Game/_Project/Characters/Heroes/DataTables/Rows/DataTabel_Character.DataTabel_Character" (`/Game/_Project/Characters/Heroes/Blueprints/GameInstance_HeroChar.CharacterDataRow` _asgame_instance_hero_char))
        (:`then`
          (bind (_charactermesh_2 _charactername_2 _animmenu_2) (break `/Game/_Project/Characters/Heroes/DataTables/Struct_Characters` _returnvalue_2))
          (set `self.Character Mesh` _charactermesh_2)
          (set `self.Character Name` _charactername_2)
          (set `self.Anim Menu` _animmenu_2)
          (goto _label))
        (:`RowNotFound`
          (`KismetSystemLibrary.PrintString` "Something Went Wrong"))))))

(fn `UserConstructionScript`)