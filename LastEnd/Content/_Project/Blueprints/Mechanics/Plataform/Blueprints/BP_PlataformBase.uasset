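; Base platform actor that lights up when something overlaps its Box trigger.
; On BeginPlay it creates a dynamic shine material shared by the Base and Plataform meshes, set to the normal glow and color.
; Overlap switches glow and color to the on-top settings and activates a particle system, while end overlap restores only the material.
; The construction script snaps Plataform to the spline's first point.
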(event `self.ReceiveBeginPlay`
  (bind _returnvalue (`KismetMaterialLibrary.CreateDynamicMaterialInstance` (`self.shineMaterial`)))
  (bind _output_get (set `self.DynamicShineMaterial` _returnvalue))
  (`PrimitiveComponent.SetMaterial` (`self.Base`) 1 _output_get)
  (`PrimitiveComponent.SetMaterial` (`self.Plataform`) 1 _output_get)
  (`MaterialInstanceDynamic.SetScalarParameterValue` (`self.DynamicShineMaterial`) "Value" (`self.normalShineValue`))
  (`MaterialInstanceDynamic.SetVectorParameterValue` (`self.DynamicShineMaterial`) "Color" (`KismetMathLibrary.Conv_ColorToLinearColor` (`self.normalColor`))))

(event `self.ReceiveActorBeginOverlap`
  (params (OtherActor :type "Actor Object Reference")))

(event `self.Box.OnComponentBeginOverlap`
  (params (OverlappedComponent :type "PrimitiveComponent Object Reference") (OtherActor :type "Actor Object Reference") (OtherComp :type "PrimitiveComponent Object Reference") (OtherBodyIndex :type Integer) (bFromSweep :type Boolean) (SweepResult :type "HitResult Structure (by ref)"))
  (`MaterialInstanceDynamic.SetScalarParameterValue` (`self.DynamicShineMaterial`) "Value" (`self.onTopShineValue`))
  (`MaterialInstanceDynamic.SetVectorParameterValue` (`self.DynamicShineMaterial`) "Color" (`KismetMathLibrary.Conv_ColorToLinearColor` (`self.onTopColor`)))
  (`ActorComponent.Activate` (`self.ParticleSystem`) false))

(event `self.Box.OnComponentEndOverlap`
  (params (OverlappedComponent :type "PrimitiveComponent Object Reference") (OtherActor :type "Actor Object Reference") (OtherComp :type "PrimitiveComponent Object Reference") (OtherBodyIndex :type Integer))
  (`MaterialInstanceDynamic.SetScalarParameterValue` (`self.DynamicShineMaterial`) "Value" (`self.normalShineValue`))
  (`MaterialInstanceDynamic.SetVectorParameterValue` (`self.DynamicShineMaterial`) "Color" (`KismetMathLibrary.Conv_ColorToLinearColor` (`self.normalColor`))))

(fn `UserConstructionScript`
  (`SceneComponent.K2_SetWorldLocation` (`self.Plataform`) (`SplineComponent.GetLocationAtSplinePoint` (`self.Spline`) 0 "World") false false))